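; Scope4x is a 4x sight Blueprint that renders a picture-in-picture magnified view on its scope mesh.
; Construction calls CreateRender, which sets a render texture as the SceneView capture target, updated every frame, and feeds it to a dynamic material on ScopeMesh.
; ZoomIn and ZoomOut step the capture's field of view, gated by comparisons with ZoomMax and ZoomMin.
; The event graph has no active logic.
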(event `self.ReceiveBeginPlay`)

(event `self.ReceiveTick`
  (params (DeltaSeconds :type "Float (single-precision)")))

(fn `CreateRender`
  (bind _sceneview (`self.SceneView`))
  ;[1 1 1] Create dynamically render texture and material for the scope 4x Scope
  (bind _output_get (set `self.TextureRender` null))
  (set `Texture.LODGroup` "TEXTUREGROUP_RenderTarget" _output_get)
  (set `SceneCaptureComponent2D.TextureTarget` (`self.TextureRender`) (`self.SceneView`))
  (set `SceneCaptureComponent.bCaptureEveryFrame` true _sceneview)
  (set `SceneCaptureComponent.bCaptureOnMovement` true _sceneview)
  (bind _returnvalue (`PrimitiveComponent.CreateDynamicMaterialInstance` (`self.ScopeMesh`) 1 "/Game/Blueprints/UI/Scope4xRender_Mat2.Scope4xRender_Mat2" "nder"))
  (bind _output_get_2 (set `self.RenderMat` _returnvalue))
  (`MaterialInstanceDynamic.SetTextureParameterValue` _output_get_2 "Alpha" (`self.TextureRender`))
  (set `self.Zoom` (`SceneCaptureComponent2D.FOVAngle` (`self.SceneView`))))

(fn `UserConstructionScript`
  (`self.CreateRender`))

(fn `ZoomIn`
  (bind _returnvalue (- (`self.Zoom`) 1.0))
  (if (> (`self.ZoomMax`) _returnvalue)
    (bind _output_get (set `self.Zoom` _returnvalue))
    (set `SceneCaptureComponent2D.FOVAngle` _output_get (`self.SceneView`))))

(fn `ZoomOut`
  (bind _returnvalue (+ (`self.Zoom`) 1.0))
  (if (> (`self.ZoomMin`) _returnvalue)
    (bind _output_get (set `self.Zoom` _returnvalue))
    (set `SceneCaptureComponent2D.FOVAngle` _output_get (`self.SceneView`))))