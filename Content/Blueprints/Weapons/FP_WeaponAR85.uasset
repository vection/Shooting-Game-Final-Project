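; AR85 first-person weapon actor for an ALS character, with muzzle flash, grip and a 4x scope.
; On BeginPlay it caches the owning character, activates the 4x scope camera, then spawns the scope from SightClass and attaches its mesh to ScopeSocket.
; UpdateCameraonScopeType switches between iron sight, Redhot and 4x cameras.
; Tick re-snaps the flash and grip to their mesh sockets every frame.
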(event `self.ReceiveTick`
  (params (DeltaSeconds :type "Float (single-precision)"))
  (bind _meshcomp (`self.MeshComp`))
  ;[1 1 1] Every Frame
  (`/Engine/EditorBlueprintResources/StandardMacros.IsValid` (`self.Mesh`)
    (:`Is Valid`
      (`SceneComponent.K2_AttachToComponent` (`self.Flash`) _meshcomp "Muzzle" "SnapToTarget" "SnapToTarget" "SnapToTarget" true)
      (`SceneComponent.K2_AttachToComponent` (`self.Grip`) _meshcomp "GripSocket" "SnapToTarget" "SnapToTarget" "SnapToTarget" true))))

(event `self.ReceiveActorBeginOverlap`
  (params (OtherActor :type "Actor Object Reference")))

(event `self.ReceiveBeginPlay`
  (bind _returnvalue (`self.GetOwner`))
  (`/Engine/EditorBlueprintResources/StandardMacros.IsValid` _returnvalue
    (:`Is Valid`
      (bind _asals_base_character (cast `/Game/Blueprints/ALS_BaseCharacter` _returnvalue))
      (set `self.ALS_BaseCharacter` _asals_base_character)
      (`self.Update Camera on ScopeType` "Scope4x")
      (`self.AttachScope`)
      (`self.SetScope`))))

(event `Update Camera on ScopeType`
  (params (`Desired Scope Type` :type "ScopeType Enum" :default "IronSight"))
  ;[1 1 1] Scope Camera (Need to be tested more)
  (switch `ScopeType` `Desired Scope Type`
    (:`IronSight`
      (`ActorComponent.SetActive` (`self.IronSightCamera`) true false)
      (`ActorComponent.SetActive` (`self.RedhotCamera`) false false)
      (`ActorComponent.SetActive` (`self.ScopeCamera`) false false))
    (:`Redhot`
      (`ActorComponent.SetActive` (`self.RedhotCamera`) true false)
      (`ActorComponent.SetActive` (`self.IronSightCamera`) false false)
      (`ActorComponent.SetActive` (`self.ScopeCamera`) false false))
    (:`Scope4x`
      (`ActorComponent.SetActive` (`self.ScopeCamera`) true false)
      (`ActorComponent.SetActive` (`self.RedhotCamera`) false false)
      (`ActorComponent.SetActive` (`self.IronSightCamera`) false false)))
  (set `self.ScopeType` `Desired Scope Type`))

(fn `AttachScope`
  (bind _asscope_4x (castclass `/Game/Blueprints/Sights/Scope4x` (`self.SightClass`)))
  (set `self.ScopeClass` _asscope_4x))

(fn `SetScope`
  (bind _returnvalue (`|SpawnActorFromClass` (`self.ScopeClass`) (`SceneComponent.GetSocketTransform` (`self.MeshComp`) "ScopeSocket" "RTS_World") "AlwaysSpawn" "OverrideRootScale" self null))
  (bind _output_get (set `self.ScopeObject` _returnvalue))
  (set `/Game/Blueprints/Sights/Scope4x.CurrentWeapon` self _output_get)
  (`self.SetOwner` _output_get (`self.ALS_BaseCharacter`))
  (bind _scopemesh (`/Game/Blueprints/Sights/Scope4x.ScopeMesh` _output_get))
  (`PrimitiveComponent.SetCollisionEnabled` _scopemesh "NoCollision")
  (`SceneComponent.K2_AttachToComponent` _scopemesh (`self.MeshComp`) "ScopeSocket" "SnapToTarget" "SnapToTarget" "SnapToTarget" true))

(fn `UserConstructionScript`)