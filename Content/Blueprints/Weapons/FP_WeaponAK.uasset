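; First-person AK weapon Blueprint, judging by its name, that assembles its flash, grip and scope on the weapon mesh.
; Tick re-attaches all three components to their mesh sockets every frame with snap rules.
; A separate FF function runs a debug-drawn line trace from the Muzzle socket location, without using the hit result.
; The trace end adds a fixed world-X offset to the unscaled forward vector, ignoring the start point.
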(event `self.ReceiveTick`
  (params (DeltaSeconds :type "Float (single-precision)"))
  (bind _meshcomp (`self.MeshComp`))
  ;[1 1 1] Every Frame
  (`SceneComponent.K2_AttachToComponent` (`self.Flash`) _meshcomp "Muzzle" "SnapToTarget" "SnapToTarget" "SnapToTarget" true)
  (`SceneComponent.K2_AttachToComponent` (`self.Grip`) _meshcomp "GripSocket" "SnapToTarget" "SnapToTarget" "SnapToTarget" true)
  (`SceneComponent.K2_AttachToComponent` (`self.Scope`) _meshcomp "ScopeSocket" "SnapToTarget" "SnapToTarget" "SnapToTarget" true))

(event `self.ReceiveActorBeginOverlap`
  (params (OtherActor :type "Actor Object Reference")))

(event `self.ReceiveBeginPlay`)

(fn `FF`
  (`KismetSystemLibrary.LineTraceSingle` :`Start` (`SceneComponent.GetSocketLocation` (`self.Flash`) "Muzzle") :`End` (+ (`KismetMathLibrary.GetForwardVector` (`self.K2_GetActorRotation`)) (5000.0 0.0 0.0)) :`TraceChannel` "TraceTypeQuery3" :`DrawDebugType` "ForDuration"))

(fn `UserConstructionScript`)