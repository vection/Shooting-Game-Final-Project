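; First-person AWM weapon Blueprint that sets up its sight cameras and attached scope.
; On BeginPlay it toggles the iron sight or scope camera by ScopeType, then resolves SightClass to a 4x or 8x scope class.
; It spawns that scope with itself as CurrentWeapon and attaches the collisionless mesh to RDS_Socket.
; Tick re-attaches the Flash and Scope components to their weapon mesh sockets every frame.
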(event `self.ReceiveTick`
  (params (DeltaSeconds :type "Float (single-precision)"))
  ;[1 1 1] Every Frame
  (`SceneComponent.K2_AttachToComponent` (`self.Flash`) (`self.MeshComp`) "Muzzle" "SnapToTarget" "SnapToTarget" "SnapToTarget" true)
  (`SceneComponent.K2_AttachToComponent` (`self.Scope`) (`self.MeshComp`) "RDS_Socket" "SnapToTarget" "SnapToTarget" "SnapToTarget" true))

(event `self.ReceiveActorBeginOverlap`
  (params (OtherActor :type "Actor Object Reference")))

(event `self.ReceiveBeginPlay`
  (`self.Update Camera on ScopeType`)
  (`self.AttachScope`)
  (`self.SetScope`))

(event `Update Camera on ScopeType`
  ;[1 1 1] Scope Camera
  (switch `ScopeType` (`self.ScopeType`)
    (:`IronSight`
      (`ActorComponent.SetActive` (`self.IronSightCamera`) true false)
      (`ActorComponent.SetActive` (`self.ScopeCamera`) false false))
    (:`Scope4x`
      (`ActorComponent.SetActive` (`self.ScopeCamera`) true false)
      (`ActorComponent.SetActive` (`self.IronSightCamera`) false false))))

(fn `AttachScope`
  (bind _asscope_4x (castclass `/Game/Blueprints/Sights/Scope4x` (`self.SightClass`))
    (:`then`
      (set `self.ScopeClass` _asscope_4x))
    (:`CastFailed`
      (bind _asscope_8x (castclass `/Game/Blueprints/Sights/Scope8x` (`self.SightClass`)))
      (set `self.ScopeClass` _asscope_8x))))

(fn `SetScope`
  (bind _returnvalue (`|SpawnActorFromClass` (`self.ScopeClass`) (`SceneComponent.GetSocketTransform` (`self.MeshComp`) "RDS_Socket" "RTS_World") "AlwaysSpawn" "OverrideRootScale" self null))
  (bind _output_get (set `self.ScopeObject` _returnvalue))
  (set `/Game/Blueprints/Sights/Scope4x.CurrentWeapon` self _output_get)
  (bind _scopemesh (`/Game/Blueprints/Sights/Scope4x.ScopeMesh` _output_get))
  (`PrimitiveComponent.SetCollisionEnabled` _scopemesh "NoCollision")
  (`SceneComponent.K2_AttachToComponent` _scopemesh (`self.MeshComp`) "RDS_Socket" "SnapToTarget" "SnapToTarget" "SnapToTarget" true))

(fn `UserConstructionScript`)