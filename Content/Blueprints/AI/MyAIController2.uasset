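; AI controller for an ALS_AICharacter that runs its behavior tree and shuts it down on death.
; On begin play it caches the possessed character and starts AI_BT.
; Each tick, once the character is dead, it stops the brain logic and the character's firing.
; A ChangeFocus function snaps control rotation to look from one point toward another.
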(event `self.ReceiveBeginPlay`
  (bind _asals_aicharacter (cast `/Game/Blueprints/ALS_AICharacter` (`self.K2_GetPawn` self)))
  (set `self.CharacterRef` _asals_aicharacter)
  (`self.RunBehaviorTree` (`AIBlueprintHelperLibrary.GetAIController` self) "/Game/Blueprints/AI/AI_BT.AI_BT"))

(event `self.ReceiveTick`
  (params (DeltaSeconds :type "Float (single-precision)"))
  (if (`FPCharacter.isDead` (`self.CharacterRef`))
    (`BrainComponent.StopLogic` (`self.BrainComponent`) "Dead")
    (`FPCharacter.StopFire` (`self.CharacterRef`))))

(fn `ChangeFocus`
  (params (FocusTo :type "Vector Structure") (`Actor vector` :type "Vector Structure"))
  (`self.SetControlRotation` self (`KismetMathLibrary.FindLookAtRotation` FocusTo `Actor vector`)))

(fn `UserConstructionScript`)