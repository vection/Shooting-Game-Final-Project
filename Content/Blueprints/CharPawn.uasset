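; CharPawn is a player character Blueprint with aim, prone, crouch and run input.
; Input toggles prone and crouch, while held keys set aiming and switch running state and walk speed.
; BeginPlay spawns an AR85 weapon onto a mesh socket and adds a crosshair widget.
; Tick and actor overlap share logic that creates and displays a new Main_Menu widget on every call, without a guard.
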(event `self.ReceiveTick`
  (params (DeltaSeconds :type "Float (single-precision)"))
  (bind _returnvalue (`|CreateWidget` "/Game/Blueprints/UI/Main_Menu.Main_Menu_C" :!label _label))
  (bind _output_get (set `self.Main_Window` _returnvalue))
  (`UserWidget.AddToViewport` _output_get 0))

(event `self.ReceiveActorBeginOverlap`
  (params (OtherActor :type "Actor Object Reference"))
  (goto _label))

(event `InputAction|Aiming`
  (params (Key :type "Key Structure"))
  (:`Pressed`
    (set `self.isAiming` true))
  (:`Released`
    (set `self.isAiming` false)))

(event `InputAction|Prone`
  (params (Key :type "Key Structure"))
  (:`Pressed`
    (if (`self.isProning`)
      (set `self.isProning` false)
      (else
        (set `self.isProning` true)))))

(event `InputAction|Crouch`
  (params (Key :type "Key Structure"))
  ;[1 1 1] Crouch
  (:`Pressed`
    (if (`self.bIsCrouched`)
      (`self.UnCrouch`)
      (else
        (`self.Crouch`)))))

(event `InputAction|Run`
  (params (Key :type "Key Structure"))
  (bind _charactermovement (`self.CharacterMovement`))
  ;[1 1 1] Run method
  (:`Pressed`
    (set `self.isRunning` true)
    (set `CharacterMovementComponent.MaxWalkSpeed` 1000.0 _charactermovement))
  (:`Released`
    (set `self.isRunning` false)
    (set `CharacterMovementComponent.MaxWalkSpeed` 600.0 _charactermovement)))

(event `self.ReceiveBeginPlay`
  ;[1 1 1] Attach to weapon
  (bind _returnvalue (`|SpawnActorFromClass` "/Game/Blueprints/Weapons/FP_WeaponAR85.FP_WeaponAR85_C" (`self.GetTransform`) "AlwaysSpawn" "OverrideRootScale" self null))
  (bind _output_get (set `self.Weapon` _returnvalue))
  (`self.K2_AttachToComponent` _output_get (`self.Mesh`) "WeaponSocketAR" "SnapToTarget" "SnapToTarget" "SnapToTarget" true)
  (bind _returnvalue_2 (`|CreateWidget` "/Game/Blueprints/UI/BP_Crosshair.BP_Crosshair_C"))
  (`UserWidget.AddToViewport` _returnvalue_2 0))

(fn `UserConstructionScript`)